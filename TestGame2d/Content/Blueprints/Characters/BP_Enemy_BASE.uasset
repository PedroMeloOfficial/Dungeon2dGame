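; Base enemy character that deals contact damage to the player and reports its removal to the spawner that owns it.
; It starts a looping sprite flicker timer and invincibility on BeginPlay, and moves through WalkTowards unless dead or stunned.
; Hits extend the parent handling with hit stop and a retriggerable stun.
; Death disables the hurtbox, then after a delay plays sound and skull explosion VFX before destroying the actor.
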(event OnComponentBeginOverlap(HurtBox)
  (params (OverlappedComponent :type Primitive%20Component%20Object%20Reference) (OtherActor :type Actor%20Object%20Reference) (OtherComp :type Primitive%20Component%20Object%20Reference) (OtherBodyIndex :type Integer) (bFromSweep :type Boolean) (SweepResult :type Hit%20Result%20Structure%20%28by%20ref%29))
  (bind _asbp_player (Utilities|Casting|CastToBP_Player OtherActor))
  (if (== (Variables|/Game/Blueprints/Characters/BP_Char_BASE.BP_Char_BASE_C|GetHurtBox _asbp_player) OtherComp)
    (Game|Damage|ApplyDamage _asbp_player (Variables|Default|GetDamage) 0 self)))

(event Custom|WalkTowards
  (params (WorldDirection :type Vector))
  (if (and (not (Variables|/Game/Blueprints/Components/BPC_Health.BPC_Health_C|GetIsDead (Variables|Default|GetBPC_Health))) (not (Variables|Default|GetIsStunned)))
    (Pawn|Input|AddMovementInput WorldDirection 1.0 false)))

(event Custom|SetStun
  (Variables|Default|SetIsStunned true)
  (Utilities|FlowControl|RetriggerableDelay (Variables|Default|GetStunedDuration))
  (Variables|Default|SetIsStunned false))

(event Custom|HandleDeath
  (Collision|SetCollisionEnabled (Variables|Default|GetHurtBox) "NoCollision")
  (Utilities|FlowControl|Delay (Variables|Default|GetDespawnDelay))
  (Audio|PlaySound2D "/Game/Sounds/S_EnemyDespawn_Cue.S_EnemyDespawn_Cue" 1.0 1.0 0.0 0 0)
  (Game|SpawnActorfromClass "/Game/Blueprints/VFX/BP_VFX_SkullExplosion.BP_VFX_SkullExplosion_C" (Math|Transform|MakeTransform (Transformation|GetActorLocation) "0, 0, 0" "1.000000,1.000000,1.000000") "AlwaysSpawn" "MultiplyWithRoot" 0 0)
  (Actor|DestroyActor))

(event EventBeginPlay
  (|CallParentFunction)
  (bind _returnvalue (Utilities|Time|SetTimerbyEvent (EventDispatchers|CreateEvent :!event SetSpriteVisibility) (Variables|Default|GetSpriteFlickerInterval) true))
  (Variables|Default|SetFlickerHandle _returnvalue)
  (Default|SetInvincibility (Variables|Default|GetBPC_Health)))

(event EventDestroyed
  (Default|OnEnemyDeath (Variables|Default|GetOwningSpawner) self))

(fn ConstructionScript
  (|CallParentFunction))

(fn HandleHitExtended
  (|CallParentFunction)
  (CallFunction|HitStop)
  (CallFunction|SetStun)
  (if (Variables|/Game/Blueprints/Components/BPC_Health.BPC_Health_C|GetIsDead (Variables|Default|GetBPC_Health))
    (CallFunction|HandleDeath)))