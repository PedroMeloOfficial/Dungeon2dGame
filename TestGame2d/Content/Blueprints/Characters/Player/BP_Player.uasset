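; Player character for a sprite-based dungeon game, with Enhanced Input movement and a sword attack that damages enemies overlapping its hitbox.
; Animation override callbacks set and clear the attack and stun flags that, with death, gate input.
; Taking a hit starts health-component invincibility and disables the hurtbox, then leads to the death animation or a looping flicker timer.
; Invincibility expiry stops the flicker and restores sprite visibility and hurtbox collision.
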(event Custom|OnInvincibilityExpired
  (Utilities|Time|ClearandInvalidateTimerbyHandle (Variables|Default|GetFlickerHandle))
  (Rendering|SetVisibility (Variables|Default|GetSprite) true false)
  (Collision|SetCollisionEnabled (Variables|Default|GetHurtBox) "QueryOnly"))

(event Input|EnhancedActionEvents|EnhancedInputActionIA_Move
  (params (ActionValue :type Vector%202D%20Structure) (ElapsedSeconds :type Float%20%28double-precision%29) (TriggeredSeconds :type Float%20%28double-precision%29) (InputAction :type Input%20Action%20Object%20Reference :default "/Game/Inputs/Actions/IA_Move.IA_Move"))
  (bind (_x _y) (Math|Vector2D|BreakVector2D ActionValue))
  (if (CallFunction|CanAct)
    (Pawn|Input|AddMovementInput "1.000000,0.000000,0.000000" _x false)
    (Pawn|Input|AddMovementInput "0.000000,1.000000,0.000000" _y false)))

(event Input|EnhancedActionEvents|EnhancedInputActionIA_Sword
  (params (ActionValue :type Boolean) (ElapsedSeconds :type Float%20%28double-precision%29) (TriggeredSeconds :type Float%20%28double-precision%29) (InputAction :type Input%20Action%20Object%20Reference :default "/Game/Inputs/Actions/IA_Sword.IA_Sword"))
  (:Started
    (if (CallFunction|CanAct)
      (|PlayAnimationOverridewithCallbacks (Variables|/Script/PaperZD.PaperZDAnimationComponent|GetAnimInstance (Variables|Default|GetAnimationComponent)) "/Game/Blueprints/Characters/Player/AnimSequences/Attack.Attack" "DefaultSlot" (Variables|Default|GetSwordPlayRate) 0.0
        (:then
          (Variables|Default|SetIsAttacking true))
        (:OnCompleted
          (Variables|Default|SetIsAttacking false :!label _label))
        (:OnCancelled
          (goto _label))))))

(event EventBeginPlay
  (Utilities|FlowControl|Sequence
    (:then_0
      (bind _asplayer_controller (Utilities|Casting|CastToPlayerController (Pawn|GetController)))
      (Input|AddMappingContext (PlayerController|LocalPlayerSubsystems|GetEnhancedInputLocalPlayerSubsystem _asplayer_controller) "/Game/Inputs/IMC_Dungeon.IMC_Dungeon" 0 "(bIgnoreAllPressedKeysUntilRelease=True,bForceImmediately=False,bNotifyUserSettings=False)"))
    (:then_1
      (EventDispatchers|BindEventtoInvincibilityExpired (Variables|Default|GetBPC_Health) (delegate Custom|OnInvincibilityExpired)))))

(event Collision|EventActorBeginOverlap
  (params (OtherActor :type Actor%20Object%20Reference)))

(event EventTick
  (params (DeltaSeconds :type Float%20%28single-precision%29)))

(event EventHandleHitExtended
  (|CallParentFunction)
  (Default|SetInvincibility (Variables|Default|GetBPC_Health))
  (Collision|SetCollisionEnabled (Variables|Default|GetHurtBox) "NoCollision")
  (|PlayAnimationOverridewithCallbacks (Variables|/Script/PaperZD.PaperZDAnimationComponent|GetAnimInstance (Variables|Default|GetAnimationComponent)) (Variables|Default|GetGetHitAnim) "DefaultSlot" 1.0 0.0
    (:then
      (Variables|Default|SetIsStunned true))
    (:OnCompleted
      (Variables|Default|SetIsStunned false :!label _label)
      (CallFunction|HitStop)
      (if (Variables|/Game/Blueprints/Components/BPC_Health.BPC_Health_C|GetIsDead (Variables|Default|GetBPC_Health))
        (Class|PaperZDAnimInstance|JumptoNode (Variables|/Script/PaperZD.PaperZDAnimationComponent|GetAnimInstance (Variables|Default|GetAnimationComponent)) "DeadJump" "None")
        (else
          (bind _returnvalue (Utilities|Time|SetTimerbyEvent (EventDispatchers|CreateEvent :!event SetSpriteVisibility) (Variables|Default|GetSpriteFlickerInterval) true))
          (Variables|Default|SetFlickerHandle _returnvalue))))
    (:OnCancelled
      (goto _label))))

(fn ConstructionScript
  (|CallParentFunction))

(fn CanAct
  (return (Math|Boolean|ANDBoolean (not (Variables|Default|GetIsStunned)) (not (Variables|/Game/Blueprints/Components/BPC_Health.BPC_Health_C|GetIsDead (Variables|Default|GetBPC_Health))) (not (Variables|Default|GetIsAttacking)))))

(fn CheckHit
  (bind _arrayelement (Utilities|Array|ReverseforEachLoop (Collision|GetOverlappingActors (Variables|Default|GetHitBox) "/Game/Blueprints/Characters/BP_Enemy_BASE.BP_Enemy_BASE_C" :!class /Script/Engine.PrimitiveComponent))
    (:LoopBody
      (Game|Damage|ApplyDamage _arrayelement (Variables|Default|GetSwordDamage) 0 self))))