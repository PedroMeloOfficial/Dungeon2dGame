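; BPC_Health is a health component that tracks current health, death and temporary invincibility for its owner.
; Health starts at maximum, and the increase and decrease functions clamp it, with decrease also updating the dead flag.
; SetInvincibility uses a retriggerable delay, so repeat calls restart the window before InvincibilityExpired is called.
; CanBeDamaged reports whether the owner is neither dead nor invincible, but DecreaseHealth does not check it.
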(event Custom|SetInvincibility
  (Variables|Default|SetIsInvincible true)
  (Utilities|FlowControl|RetriggerableDelay (Variables|Default|GetInvicibilityDuration))
  (Variables|Default|SetIsInvincible false)
  (Default|CallInvincibilityExpired))

(event EventBeginPlay
  (Variables|Default|SetCurrentHealth (Variables|Default|GetMaxHealth)))

(fn DecreaseHealth
  (params (Amount :type Float%20%28double-precision%29))
  (Variables|Default|SetCurrentHealth (Math|Float|Max(Float) (- (Variables|Default|GetCurrentHealth) Amount) 0.0))
  (Variables|Default|SetIsDead (<= (Variables|Default|GetCurrentHealth) 0.0))
  (return))

(fn CanbeDamaged
  (return (and (not (Variables|Default|GetIsDead)) (not (Variables|Default|GetIsInvincible)))))

(fn IncreaseHealth
  (params (Amount :type Float%20%28double-precision%29))
  (Variables|Default|SetCurrentHealth (Math|Float|Min(Float) (+ (Variables|Default|GetCurrentHealth) Amount) (Variables|Default|GetMaxHealth))))