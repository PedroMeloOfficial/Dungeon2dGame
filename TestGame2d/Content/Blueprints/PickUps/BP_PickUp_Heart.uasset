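; BP_PickUp_Heart is a heart pickup that heals the player.
; It overrides HandlePickUp to run the parent logic, then call GetHealed on the player with HealAmount.
; ActorBeginOverlap and construction only forward to the parent class, and BeginPlay and Tick are disabled stubs.
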(event EventBeginPlay
  (|CallParentFunction) ; This node is disabled and will not be called.\nDrag off pins to build functionality.
)

(event Collision|EventActorBeginOverlap
  (params (OtherActor :type Actor%20Object%20Reference))
  (|CallParentFunction 0))

(event EventTick
  (params (DeltaSeconds :type Float%20%28single-precision%29))
  (|CallParentFunction DeltaSeconds) ; This node is disabled and will not be called.\nDrag off pins to build functionality.
)

(fn ConstructionScript
  (|CallParentFunction))

(fn HandlePickUp
  (params (BP_Player :type BP%20Player%20Object%20Reference))
  (|CallParentFunction BP_Player)
  (Default|GetHealed BP_Player (Variables|Default|GetHealAmount))
  (return))